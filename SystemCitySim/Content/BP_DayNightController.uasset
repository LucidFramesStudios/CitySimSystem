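; Day/night controller that drives a referenced Sunlight actor from the world time in WorldSimulationSubsystem.
; Each Tick it snaps the sun to a fixed pitch, with yaw making one full turn over the 24-hour clock.
; Light intensity follows a half sine that peaks at midday and is floored so night keeps a dim light.
; An unconnected Timeline and several unused interpolation and rotation experiments remain in the graph.
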(event EventBeginPlay)

(event Collision|EventActorBeginOverlap
  (params (OtherActor :type Actor%20Object%20Reference)))

(event EventTick
  (params (DeltaSeconds :type Float%20%28single-precision%29))
  (bind _returnvalue (Subsystems|GetWorldSimulationSubsystem))
  (bind _sunlight (Variables|Default|GetSunlight))
  (bind _returnvalue_2 (Class|WorldSimulationSubsystem|GetWorldTime _returnvalue))
  (bind _returnvalue_3 (/ _returnvalue_2 24.0))
  (Transformation|SetActorRotation _sunlight (Math|Rotator|SelectRotator "4.000000,356.000000,0.000000" (Math|Rotator|MakeRotator 0.0 -46.0 (* _returnvalue_3 3.6e+02)) false))
  (Rendering|Components|Light|SetIntensity (Variables|/Script/Engine.Light|GetLightComponent _sunlight) (* (Math|Float|Max(Float) (Math|Trig|Sin(Degrees) (* _returnvalue_3 1.8e+02)) 0.1) 5.0)))

(fn ConstructionScript)